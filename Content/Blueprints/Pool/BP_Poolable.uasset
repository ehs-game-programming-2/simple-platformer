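; BP_Poolable is a poolable actor that can be switched on and off, apparently for reuse by an object pool.
; Release and Enable only broadcast the OnObjectReleased and OnObjectEnabled dispatchers, leaving any response to bound listeners.
; Toggle sets visibility, actor tick and collision together from one boolean.
; IsEnabled derives the active state from the actor's hidden flag, with no separate state variable.
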(fn `Enable`
  (`self.OnObjectEnabled` self))

(fn `Is Enabled`
  (returns (value :type Boolean))
  (return (not (`self.bHidden`))))

(fn `Release`
  (`self.OnObjectReleased` self))

(fn `Toggle`
  (params (Value :type Boolean))
  (`self.SetActorHiddenInGame` (not Value))
  (`self.SetActorTickEnabled` Value)
  (`self.SetActorEnableCollision` Value))

(fn `UserConstructionScript`)