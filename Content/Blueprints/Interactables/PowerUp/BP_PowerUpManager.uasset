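; BP_PowerUpManager handles speed power-ups, changing the walk speed of the player who takes one.
; On BeginPlay it finds every BP_PowerUp in the level and binds to each one's taken event.
; PowerUpCollected saves the old speed and applies the power-up's new speed.
; It starts a duration timer with no bound event, so restoring speed and disabling the pickup follow immediately rather than on expiry.
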(event `self.ReceiveBeginPlay`
  (bind _outactors (`GameplayStatics.GetAllActorsOfClass` "/Game/Blueprints/Interactables/PowerUp/BP_PowerUp.BP_PowerUp_C"))
  (bind _output_get (set `self.PowerUps` _outactors))
  (for _array_element _output_get
    (add `/Game/Blueprints/Interactables/PowerUp/BP_PowerUp.OnPowerUpTaken` _array_element (delegate `OnPowerUpTaken_Event`))))

(event `OnPowerUpTaken_Event`
  (params (powerUP :type "/Game/Blueprints/Interactables/PowerUp/BP_PowerUp Object Reference") (Player :type "/Game/Blueprints/Character/BP_Player Object Reference"))
  (`self.PowerUpCollected` powerUP Player))

(fn `NewFunction`)

(fn `PowerUpCollected`
  (params (PowerUp :type "/Game/Blueprints/Interactables/PowerUp/BP_PowerUp Object Reference") (player :type "/Game/Blueprints/Character/BP_Player Object Reference"))
  (locals (powerUPLocal :type "/Game/Blueprints/Interactables/PowerUp/BP_PowerUp Object Reference") (playerLocal :type "/Game/Blueprints/Character/BP_Player Object Reference"))
  (bind _charactermovement (`Character.CharacterMovement` (`local.playerLocal`)))
  (set `local.powerUPLocal` PowerUp)
  (set `local.playerLocal` player)
  (set `/Game/Blueprints/Interactables/PowerUp/BP_PowerUp.OldSpeed` (`MovementComponent.GetMaxSpeed` _charactermovement) (`local.powerUPLocal`))
  (set `CharacterMovementComponent.MaxWalkSpeed` (`/Game/Blueprints/Interactables/PowerUp/BP_PowerUp.NewSpeed` (`local.powerUPLocal`)) _charactermovement)
  (`KismetSystemLibrary.K2_SetTimerDelegate` :`Time` (`/Game/Blueprints/Interactables/PowerUp/BP_PowerUp.PowerUpDuration` (`local.powerUPLocal`)))
  (set `CharacterMovementComponent.MaxWalkSpeed` (`self.OldSpeed`) (`Character.CharacterMovement` (`local.playerLocal`)))
  (`/Game/Blueprints/Interactables/PowerUp/BP_PowerUp.DisableActor` (`local.powerUPLocal`)))

(fn `UserConstructionScript`)