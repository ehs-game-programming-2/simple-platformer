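; Collectible power-up actor that spins and bobs in place until a player collects it.
; On BeginPlay, one timeline loops a full yaw rotation while another ping-pongs the height 30 units above the starting Z.
; Collect broadcasts OnPowerUpTaken with itself and the player, without disabling the actor.
; A separate DisableActor function, not called within this Blueprint, hides it and switches off tick and collision.
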(event `self.ReceiveBeginPlay`
  (`self.Start Rotation`)
  (`self.InizializeLocalVariables`)
  (`self.Start Location`))

(event `Start Rotation`
  ;[0.0388 0.15 0.1135 0.5] Rotation
  (bind (_direction _value) (`Timeline|Timeline` :!via `PlayFromStart` :!label _label)
    (:`Update`
      (`self.K2_SetActorRelativeRotation` (`KismetMathLibrary.MakeRotator` 0.0 0.0 (`KismetMathLibrary.Lerp` 0.0 360.0 _value))))
    (:`Finished`
      (switch `ETimelineDirection` _direction
        (:`Forward`
          (`self.Start Rotation`))
        (:`Backward`
          (`self.Reverse Rotation`))))))

(event `Reverse Rotation`
  ;[0.0388 0.15 0.1135 0.5] Rotation
  (goto _label :!via `ReverseFromEnd`))

(event `Start Location`
  (bind (_returnvalue_x _returnvalue_y) (`KismetMathLibrary.BreakVector` (`self.K2_GetActorLocation`)))
  ;[0.05237 0.08523 0.15 0.5] Position
  (bind (_direction _value) (`Timeline|Timeline_0` :!via `PlayFromStart` :!label _label_2)
    (:`Update`
      (`self.K2_SetActorRelativeLocation` (`KismetMathLibrary.MakeVector` _returnvalue_x _returnvalue_y (`KismetMathLibrary.Lerp` (`self.Start Locat`) (`self.EndLocation`) _value))))
    (:`Finished`
      (switch `ETimelineDirection` _direction
        (:`Forward`
          (`self.Reverse Location`))
        (:`Backward`
          (`self.Start Location`))))))

(event `Reverse Location`
  ;[0.05237 0.08523 0.15 0.5] Position
  (goto _label_2 :!via `ReverseFromEnd`))

(event `/Game/Blueprints/Interactables/BPI_IInteractable.Collect`
  (params (Player :type "/Game/Blueprints/Character/BP_Player Object Reference"))
  (`self.OnPowerUpTaken` self Player))

(fn `DisableActor`
  (`self.SetActorHiddenInGame` true)
  (`self.SetActorTickEnabled` false)
  (`self.SetActorEnableCollision` false))

(fn `InizializeLocalVariables`
  (bind (_returnvalue_x _returnvalue_y _returnvalue_z) (`KismetMathLibrary.BreakVector` (`self.K2_GetActorLocation`)))
  (bind _output_get (set `self.Start Locat` _returnvalue_z))
  (set `self.EndLocation` (+ _output_get 30.0)))

(fn `UserConstructionScript`)