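; BP_LiftManager is a manager for BP_Lift actors, meant to move a lift out and back when started.
; LiftStart_Event plays the UpAndDown timeline to offset the given lift along world Y from its old location, then reverses it once.
; The code that finds all lifts, binds their LiftStart dispatchers and calls Collect is unconnected, and BeginPlay is empty, so nothing here hooks up the event.
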(event `self.ReceiveBeginPlay`)

(event `LiftStart_Event`
  (params (Lift :type "/Game/Blueprints/Interactables/Lift/BP_Lift Object Reference") (oldLocation :type "Vector Structure"))
  (bind (_direction _lift) (`Timeline|Up and Down` :!via `PlayFromStart` :!label _label)
    (:`Update`
      (`self.K2_SetActorLocation` Lift (+ (* _lift (0.0 1.0 0.0)) oldLocation) false false))
    (:`Finished`
      (switch `ETimelineDirection` _direction
        (:`Forward`
          (goto _label :!via `ReverseFromEnd`))))))

(fn `UserConstructionScript`)