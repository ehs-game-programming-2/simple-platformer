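; BP_Lift is a lift actor that moves vertically back and forth in a continuous loop from BeginPlay.
; A timeline lerps the actor between its starting location and that point raised by Higth, reversing or replaying each time it finishes.
; A Collect event re-records the current location as the base position and calls LiftStart with the lift and that location.
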(event `self.ReceiveBeginPlay`
  (bind _returnvalue_location (`KismetMathLibrary.BreakTransform` (`self.GetTransform`)))
  (bind _output_get (set `self.oldPos` _returnvalue_location))
  (bind (_direction _lift) (`Timeline|Timeline` :!label _label)
    (:`Update`
      (`self.K2_SetActorLocation` (`KismetMathLibrary.VLerp` _output_get (+ _output_get (`KismetMathLibrary.MakeVector` 0.0 0.0 (`self.Higth`))) _lift)))
    (:`Finished`
      (switch `ETimelineDirection` _direction
        (:`Forward`
          (goto _label :!via `ReverseFromEnd`))
        (:`Backward`
          (goto _label :!via `PlayFromStart`))))))

(event `/Game/Blueprints/Interactables/BPI_IInteractable.Collect`
  (params (Player :type "/Game/Blueprints/Character/BP_Player Object Reference"))
  (bind _returnvalue_location (`KismetMathLibrary.BreakTransform` (`self.GetTransform`)))
  (bind _output_get (set `self.oldPos` _returnvalue_location))
  (`self.LiftStart` self _output_get))

(fn `UserConstructionScript`)