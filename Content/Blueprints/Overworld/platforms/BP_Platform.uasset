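; Moving platform actor for the overworld that loops endlessly through a list of waypoints from BeginPlay.
; Locations are relative offsets, resolved against the StartLocation captured at BeginPlay, and the index wraps to zero after the last.
; A Timeline lerps the actor to each waypoint without sweep, and its Finished event re-calls PlayTimeline for the next leg.
; SwapLocations and Initialize Locations are not called in these graphs.
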(event `self.ReceiveBeginPlay`
  (set `self.Start Location` (`self.K2_GetActorLocation`))
  (`self.Play Timeline` (`self.Start Location`) (`self.Get Location Current At Index`)))

(event `Play Timeline`
  (params (`Start Location` :type "Vector Structure") (`End Location` :type "Vector Structure"))
  (bind (_direction _value) (`Timeline|Timeline` :!via `PlayFromStart`)
    (:`Update`
      (`self.K2_SetActorLocation` (`KismetMathLibrary.VLerp` `Start Location` `End Location` _value)))
    (:`Finished`
      (`/Engine/EditorBlueprintResources/StandardMacros.IncrementInt` (`self.Current Index`)
        (:`  `
          (`self.Play Timeline` (`self.K2_GetActorLocation`) (`self.Get Location Current At Index`)))))))

(fn `Get Location Current At Index`
  (returns (Location :type "Vector Structure"))
  (bind _locations (`self.Locations`))
  (bind _start_location (`self.Start Location`))
  (if (!= (`self.Current Index`) (`KismetArrayLibrary.Array_Length` _locations))
    (return (`/Game/Blueprints/Libraries/BPFL_Transforms.Get Adjusted Location` _start_location (`|GetArrayItem` (`self.Locations`) (`self.Current Index`))))
    (else
      (set `self.Current Index` 0)
      (return (`/Game/Blueprints/Libraries/BPFL_Transforms.Get Adjusted Location` _start_location (`|GetArrayItem` _locations))))))

(fn `Swap Locations`
  (params (`Start Initial` :type "Vector Structure") (`End Initial` :type "Vector Structure"))
  (returns (Start :type "Vector Structure") (End :type "Vector Structure"))
  (return `End Initial` `Start Initial`))

(fn `UserConstructionScript`)