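; BP_Player is the player character for a coin minigame, with movement, jumping, mouse yaw and item collection.
; On BeginPlay it binds movement handlers to axis events on PC_CoinMinigame, then creates and enters a UOBJ_Defend state object.
; Capsule overlaps send CollectMessage to actors implementing BPI_ICollectible.
; The construction script draws a debug circle around the actor.
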(event `self.ReceiveBeginPlay`
  (bind _aspc_coin_minigame (cast `/Game/Blueprints/Character/PC_CoinMinigame` (`GameplayStatics.GetPlayerController` 0)))
  (add `/Game/Blueprints/Character/PC_CoinMinigame.OnAxisHorizontalEvent` _aspc_coin_minigame (delegate `on Horizontal Move`))
  (add `/Game/Blueprints/Character/PC_CoinMinigame.OnAxisVerticalEvent` _aspc_coin_minigame (delegate `On Vertical Move`))
  (bind _returnvalue (`|GenericCreateObject` "/Game/Blueprints/Character/States/UOBJ_Defend.UOBJ_Defend_C"))
  (bind _output_get (set `self.Current State` _returnvalue))
  (`/Game/Blueprints/Character/States/UOBJ_State.On Enter` _output_get))

(event `On Vertical Move`
  (params (Value :type "Float (double-precision)"))
  ;[1 0.2572 0.4382] Inputs
  (`self.AddMovementInput` (`self.GetActorForwardVector`) Value))

(event `InputAction|Jump`
  (params (Key :type "Key Structure"))
  ;[1 0.2572 0.4382] Inputs
  (:`Pressed`
    (`self.Jump`)))

(event `on Horizontal Move`
  (params (Value :type "Float (double-precision)"))
  ;[1 0.2572 0.4382] Inputs
  (`self.AddMovementInput` (`self.GetActorRightVector`) Value))

(event `InputAxis|Mouse Rotation`
  (params (AxisValue :type "Float (single-precision)"))
  ;[1 0.2572 0.4382] Inputs
  (`self.AddControllerYawInput` AxisValue))

(event `self.CapsuleComponent.OnComponentBeginOverlap`
  (params (OverlappedComponent :type "PrimitiveComponent Object Reference") (OtherActor :type "Actor Object Reference") (OtherComp :type "PrimitiveComponent Object Reference") (OtherBodyIndex :type Integer) (bFromSweep :type Boolean) (SweepResult :type "HitResult Structure (by ref)"))
  (if (`KismetSystemLibrary.DoesImplementInterface` OtherActor "/Game/Blueprints/Interactables/Coins/BPI_ICollectible.BPI_ICollectible_C")
    (message `/Game/Blueprints/Interactables/Coins/BPI_ICollectible.Collect` OtherActor self)))

(fn `GetVectorWithInput`
  (params (X :type "Float (double-precision)") (Y :type "Float (double-precision)"))
  (returns (ReturnValue :type "Vector Structure"))
  (return (`KismetMathLibrary.MakeVector` X Y)))

(fn `Is Moving`
  (params (X :type "Float (double-precision)") (Y :type "Float (double-precision)"))
  (returns (ReturnValue :type Boolean))
  (return (or (!= X 0.0) (!= Y 0.0))))

(fn `UserConstructionScript`
  (`KismetSystemLibrary.DrawDebugCircle` (`self.K2_GetActorLocation`) 100.0 12 (struct :`R` 1.0 :`G` 1.0 :`B` 1.0 :`A` 1.0) 0.0 2.0))